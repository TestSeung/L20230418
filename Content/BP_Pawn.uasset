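; Player pawn for a propeller-driven craft that pitches and rolls from input and spins its left and right propellers.
; The Enhanced Input action IA_PitchRoll supplies a 2D value that applies frame-time-scaled local roll and pitch to the actor.
; Tick calls a shared RotatePropeller custom event for each propeller, spinning it at a constant delta-time-based rate.
; Two unconnected rotation nodes for separate pitch and roll remain unused, and the graph has no translation logic.
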(event Custom|RotatePropeller
  (params (Where :type Static%20Mesh%20Component%20Object%20Reference))
  ;[1 1 1] 커스텀 이벤트
  (Transformation|AddLocalRotation Where (Math|Rotator|MakeRotator (* (Utilities|Time|GetWorldDeltaSeconds) 3.6e+03) 0.0 0.0) false false))

(event Input|EnhancedActionEvents|EnhancedInputActionIA_Pitch
  (params (ActionValue :type Float%20%28double-precision%29) (ElapsedSeconds :type Float%20%28double-precision%29) (TriggeredSeconds :type Float%20%28double-precision%29) (InputAction :type Input%20Action%20Object%20Reference :default "/Game/Input/IA_Pitch.IA_Pitch")))

(event Input|EnhancedActionEvents|EnhancedInputActionIA_Roll
  (params (ActionValue :type Float%20%28double-precision%29) (ElapsedSeconds :type Float%20%28double-precision%29) (TriggeredSeconds :type Float%20%28double-precision%29) (InputAction :type Input%20Action%20Object%20Reference :default "/Game/Input/IA_Roll.IA_Roll")))

(event Input|EnhancedActionEvents|EnhancedInputActionIA_PitchRoll
  (params (ActionValue :type Vector%202D%20Structure) (ElapsedSeconds :type Float%20%28double-precision%29) (TriggeredSeconds :type Float%20%28double-precision%29) (InputAction :type Input%20Action%20Object%20Reference :default "/Game/Input/IA_PitchRoll.IA_PitchRoll"))
  (:Triggered
    (Transformation|AddActorLocalRotation (* (Math|Rotator|MakeRotator (.x ActionValue) (.y ActionValue) 0.0) (Utilities|Time|GetWorldDeltaSeconds) 6e+01) false false)))

(event Input|EnhancedActionEvents|EnhancedInputActionIA_Fire
  (params (ActionValue :type Boolean) (ElapsedSeconds :type Float%20%28double-precision%29) (TriggeredSeconds :type Float%20%28double-precision%29) (InputAction :type Input%20Action%20Object%20Reference :default "/Game/Input/IA_Fire.IA_Fire")))

(event EventTick
  (params (DeltaSeconds :type Float%20%28single-precision%29))
  (CallFunction|RotatePropeller (Variables|Default|GetLeft))
  (CallFunction|RotatePropeller (Variables|Default|GetRight)))

(fn ConstructionScript)